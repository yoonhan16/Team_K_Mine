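; BP_ElevatorButton is an interactable elevator button that opens the elevator only once the character has done its task.
; Interact reads DidTask on BP_ThirdPersonCharacter and, if true, calls OpenElevatorDoor on BP_Elevator with the interacting player.
; Otherwise it turns off BP_Light2 and collapses BP_CollapsingFloor1, finding each target by GetActorOfClass.
; An unconnected loop that matches BP_ElevatorDoor actors to ButtonValue never runs.
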(event EventInteract
  (params (Player :type Character%20Object%20Reference))
  (bind _returnvalue (Actor|GetActorOfClass "/Game/ThirdPerson/Blueprints/BP_ThirdPersonCharacter.BP_ThirdPersonCharacter_C"))
  (if (Variables|/Game/ThirdPerson/Blueprints/BP_ThirdPersonCharacter.BP_ThirdPersonCharacter_C|GetbDidTask? _returnvalue)
    (Development|PrintString "true")
    (bind _returnvalue_2 (Actor|GetActorOfClass "/Game/Blueprints/BP_Elevator.BP_Elevator_C"))
    (Default|OpenElevatorDoor _returnvalue_2 Player)
    (else
      (Development|PrintString "false")
      (Utilities|FlowControl|Sequence
        (:then_0
          (bind _returnvalue_3 (Actor|GetActorOfClass "/Game/Blueprints/BP_Light2.BP_Light2_C"))
          (Default|LightsOff _returnvalue_3))
        (:then_1
          (bind _returnvalue_4 (Actor|GetActorOfClass "/Game/Blueprints/BP_CollapsingFloor1.BP_CollapsingFloor1_C"))
          (Default|Collapse _returnvalue_4))))))

(fn ConstructionScript)