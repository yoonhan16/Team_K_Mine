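; Elevator actor with two sliding doors that carries its platform up a fixed vertical path when a player interacts.
; Open and close events drive separate timelines that lerp both doors' relative positions in opposite directions.
; Interact starts closing the doors and the ascent together, using hardcoded world coordinates, then reopens the doors on arrival.
; Ending overlap with the player detection component reverses the opening timeline to shut the doors.
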(event OnComponentEndOverlap(PlayerOverlap)
  (params (OverlappedComponent :type Primitive%20Component%20Object%20Reference) (OtherActor :type Actor%20Object%20Reference) (OtherComp :type Primitive%20Component%20Object%20Reference) (OtherBodyIndex :type Integer))
  (bind _newtrack_0 (Timeline|Timeline ReverseFromEnd)
    (:Update
      (Utilities|FlowControl|Sequence
        (:then_0
          (Transformation|SetRelativeLocation (Variables|Default|GetRightDoor) (Math|Vector|MakeVector -5.2e+02 (Math|Float|Lerp -1e+02 -205.0 _newtrack_0) 0.0) false false))
        (:then_1
          (Transformation|SetRelativeLocation (Variables|Default|GetLeftDoor) (Math|Vector|MakeVector -5.2e+02 (Math|Float|Lerp 1e+02 205.0 _newtrack_0) 0.0) false false))))))

(event Custom|Open%20Elevator%20Door
  (params (Player :type Actor%20Object%20Reference))
  (bind _newtrack_0 (Timeline|Timeline PlayFromStart)
    (:Update
      (Utilities|FlowControl|Sequence
        (:then_0
          (Transformation|SetRelativeLocation (Variables|Default|GetRightDoor) (Math|Vector|MakeVector -5.2e+02 (Math|Float|Lerp -1e+02 -205.0 _newtrack_0) 0.0) false false))
        (:then_1
          (Transformation|SetRelativeLocation (Variables|Default|GetLeftDoor) (Math|Vector|MakeVector -5.2e+02 (Math|Float|Lerp 1e+02 205.0 _newtrack_0) 0.0) false false))))))

(event Custom|Close%20Elevator%20Door
  (params (Player :type Actor%20Object%20Reference))
  (bind _newtrack_0 (Timeline|Timeline_0 PlayFromStart)
    (:Update
      (Utilities|FlowControl|Sequence
        (:then_0
          (Transformation|SetRelativeLocation (Variables|Default|GetRightDoor) (Math|Vector|MakeVector -5.2e+02 (Math|Float|Lerp -205.0 -1e+02 _newtrack_0) 0.0) false false))
        (:then_1
          (Transformation|SetRelativeLocation (Variables|Default|GetLeftDoor) (Math|Vector|MakeVector -5.2e+02 (Math|Float|Lerp 205.0 1e+02 _newtrack_0) 0.0) false false))))))

(event EventInteract
  (params (Player :type Character%20Object%20Reference))
  (CallFunction|CloseElevatorDoor Player)
  (bind _newtrack_0 (Timeline|Timeline_1 PlayFromStart)
    (:Update
      (Transformation|SetWorldLocation (Variables|Default|GetElevator) (Math|Vector|MakeVector 895.0 2.26e+03 (Math|Float|Lerp 1.6e+03 2.8e+03 _newtrack_0)) false false))
    (:Finished
      (CallFunction|OpenElevatorDoor))))

(fn ConstructionScript)