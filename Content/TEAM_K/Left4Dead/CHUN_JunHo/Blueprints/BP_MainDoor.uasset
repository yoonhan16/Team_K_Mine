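; BP_MainDoor is an interactable double door that swings open and closed.
; Interact toggles between Open and Close using an IsInteracted flag.
; Each event plays its own Timeline, lerping the left and right door yaw in opposite directions by a quarter turn.
; Both doors lose collision while swinging and regain query and physics collision when the timeline finishes.
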(event Custom|Open
  (bind _leftdoor (Variables|Default|GetLeftDoor))
  (bind _newtrack_0 (Timeline|Timeline PlayFromStart)
    (:Update
      (Transformation|SetRelativeRotation _leftdoor (Math|Rotator|MakeRotator 0.0 0.0 (Math|Float|Lerp 0.0 -9e+01 _newtrack_0)) false false)
      (Transformation|SetRelativeRotation (Variables|Default|GetRightDoor) (Math|Rotator|MakeRotator 0.0 0.0 (Math|Float|Lerp 0.0 9e+01 _newtrack_0)) false false)
      (Collision|SetCollisionEnabled _leftdoor "NoCollision"))
    (:Finished
      (Collision|SetCollisionEnabled _leftdoor "QueryAndPhysics"))))

(event Custom|Close
  (bind _rightdoor (Variables|Default|GetRightDoor))
  (bind _leftdoor (Variables|Default|GetLeftDoor))
  (bind _newtrack_0 (Timeline|Timeline_0 PlayFromStart)
    (:Update
      (Transformation|SetRelativeRotation _leftdoor (Math|Rotator|MakeRotator 0.0 0.0 (Math|Float|Lerp -9e+01 0.0 _newtrack_0)) false false)
      (Transformation|SetRelativeRotation _rightdoor (Math|Rotator|MakeRotator 0.0 0.0 (Math|Float|Lerp 9e+01 0.0 _newtrack_0)) false false)
      (Collision|SetCollisionEnabled _rightdoor "NoCollision"))
    (:Finished
      (Collision|SetCollisionEnabled _leftdoor "QueryAndPhysics"))))

(event EventInteract
  (params (Player :type Character%20Object%20Reference))
  (if (Variables|Default|GetbIsInteracted?)
    (CallFunction|Close)
    (Variables|Default|SetbIsInteracted? false)
    (else
      (CallFunction|Open)
      (Variables|Default|SetbIsInteracted? true))))

(fn ConstructionScript)